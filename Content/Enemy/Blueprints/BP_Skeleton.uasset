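; Skeleton enemy character that runs a behavior tree and fights the player with a sword spawned into its hand socket.
; Pawn sensing, an escape radius and damage events set a blackboard behavior enum that drives the AI.
; Damage updates the health bar and plays hit or death montages, with death stopping AI and releasing player lock-on.
; It also exposes random attack montages, lock-on indicators and hit-actor clearing for its trace component.
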(event OnSeePawn(PawnSensing)
  (params (Pawn :type Pawn%20Object%20Reference))
  ;[0.05521 0.05521 0.05521] Handle Enemy Vision
  (if (and (== Pawn (Game|GetPlayerCharacter 0)) (Utilities|Enum|NotEqual(Enum) (Variables|Default|GetBehaviour) "NewEnumerator0"))
    (Variables|Default|SetBehaviour "NewEnumerator3")
    (AI|Components|Blackboard|SetValueasEnum (AI|GetBlackboard 0) (Utilities|Name|MakeLiteralName "EBehaviour") (Variables|Default|GetBehaviour))))

(event OnComponentEndOverlap(EscapeRadius)
  (params (OverlappedComponent :type Primitive%20Component%20Object%20Reference) (OtherActor :type Actor%20Object%20Reference) (OtherComp :type Primitive%20Component%20Object%20Reference) (OtherBodyIndex :type Integer))
  ;[0.1094 0.1094 0.1094] Escape Enemy
  (Utilities|Casting|CastToBP_ThirdPersonCharacter OtherActor)
  (Variables|Default|SetBehaviour "NewEnumerator1")
  (AI|Components|Blackboard|SetValueasEnum (AI|GetBlackboard 0) (Utilities|Name|MakeLiteralName "EBehaviour") (Variables|Default|GetBehaviour))
  (Rendering|SetVisibility (Variables|Default|GetHealthBar) false false))

(event Custom|Attack
  ;[0.126 0.126 0.126] Attck System
  (bind _returnvalue (Animation|PlayAnimMontage (.OutItem (Utilities|Array|Random (Variables|Default|GetAttackAnimation))) 1.0 "None"))
  (Variables|Default|SetAttackLength _returnvalue))

(event Custom|ClearHitActors
  ;[0.05521 0.05521 0.05521] Clear Hit Actors
  (Utilities|Array|Clear (Variables|/Game/Equipments/TraceComponent.TraceComponent_C|GetActorsToIgnore (Variables|Default|GetTraceComponent))))

(event EventBeginPlay
  ;[0.101 0.101 0.101] Enemy character setup
  (Variables|Default|SetCurrentHealth (Variables|Default|GetMaxHealth))
  (AI|RunBehaviorTree (AI|GetAIController self) "/Game/Enemy/BehaviouralPatterns/SkeletonBehviourTree.SkeletonBehviourTree")
  (bind _returnvalue (Game|SpawnActorfromClass (Variables|Default|GetSword) (Transformation|GetSocketTransform (Variables|Character|GetMesh) "RightHandSocket" "RTS_World") "Undefined" "MultiplyWithRoot" 0 0))
  (bind _output_get (Variables|Default|SetSwordReference _returnvalue))
  (Transformation|AttachComponentToComponent _output_get (Variables|Character|GetMesh) "RightHandSocket" "SnapToTarget" "SnapToTarget" "SnapToTarget" true)
  (Variables|/Game/Equipments/TraceComponent.TraceComponent_C|SetSwordReference (Variables|Default|GetTraceComponent) (Variables|Default|GetSwordReference))
  (bind _asbp_third_person_character (Utilities|Casting|CastToBP_ThirdPersonCharacter (Game|GetPlayerCharacter 0)))
  (Variables|Default|SetPlayerReference _asbp_third_person_character)
  (AI|Components|Blackboard|SetValueasEnum (AI|GetBlackboard 0) (Utilities|Name|MakeLiteralName "EBehaviour") (Variables|Default|GetBehaviour))
  (Variables|/Game/Equipments/RotatingComponent.RotatingComponent_C|SetTarget (Variables|Default|GetRotatingComponent) (Game|GetPlayerCharacter 0))
  (bind _outactors (Actor|GetAllActorswithTag "Enemy"))
  (Variables|/Game/Equipments/TraceComponent.TraceComponent_C|SetEnemy (Variables|Default|GetTraceComponent) _outactors)
  (bind _asbp_skeleton_health_bar (Utilities|Casting|CastToBP_SkeletonHealthBar (UserInterface|GetWidget (Variables|Default|GetHealthBar))))
  (bind _output_get_2 (Variables|Default|SetHealthBarReference _asbp_skeleton_health_bar))
  (Variables|/Game/Enemy/Blueprints/BP_SkeletonHealthBar.BP_SkeletonHealthBar_C|SetSkeletonReference _output_get_2 self))

(event Collision|EventActorBeginOverlap
  (params (OtherActor :type Actor%20Object%20Reference)))

(event EventTick
  (params (DeltaSeconds :type Float%20%28single-precision%29)))

(event Game|Damage|EventAnyDamage
  (params (Damage :type Float%20%28single-precision%29) (DamageType :type Damage%20Type%20Object%20Reference) (InstigatedBy :type Controller%20Object%20Reference) (DamageCauser :type Actor%20Object%20Reference))
  (bind _playerreference (Variables|Default|GetPlayerReference))
  (bind _targetactor (Variables|/Game/ThirdPerson/Blueprints/BP_ThirdPersonCharacter.BP_ThirdPersonCharacter_C|GetTargetActor _playerreference))
  ;[0.1177 0.1177 0.1177] Damage System
  (Variables|Default|SetBehaviour "NewEnumerator0")
  (AI|Components|Blackboard|SetValueasEnum (AI|GetBlackboard 0) (Utilities|Name|MakeLiteralName "EBehaviour") (Variables|Default|GetBehaviour))
  (bind _output_get (Variables|Default|SetCurrentHealth (- (Variables|Default|GetCurrentHealth) Damage)))
  (if (<= _output_get 0.0)
    (Utilities|FlowControl|DoOnce false
      (:Completed
        (Default|ClearEnemies (Variables|Default|GetPlayerReference))
        (Collision|SetCollisionEnabled (Variables|Collision|GetCapsuleComponent) "NoCollision")
        (Rendering|SetVisibility (Variables|Default|GetHealthBar) false false)
        (AI|Logic|StopLogic (Variables|/Script/AIModule.AIController|GetBrainComponent (AI|GetAIController self)) "die")
        (Variables|Default|SetEnemyDead true)
        (Animation|PlayAnimMontage "/Game/Enemy/Animations/SkeleDeath_Montage.SkeleDeath_Montage" 1.0 "None")
        (Utilities|IsValid _targetactor
          (:Is%20Valid
            (if (== _targetactor self)
              (Default|DisengageLockon (Variables|Default|GetPlayerReference)))))))
    (else
      (Rendering|SetVisibility (Variables|Default|GetHealthBar) true false)
      (Default|UpdateHealthBar (Variables|Default|GetHealthBarReference))
      (Components|Movement|StopMovementImmediately (Variables|Character|GetCharacterMovement))
      (bind _returnvalue (Animation|PlayAnimMontage "/Game/Enemy/Animations/Skele_Hit_Montage.Skele_Hit_Montage" 1.0 "None"))
      (Utilities|FlowControl|RetriggerableDelay _returnvalue)
      (Variables|Default|SetBehaviour "NewEnumerator3")
      (AI|Components|Blackboard|SetValueasEnum (AI|GetBlackboard 0) (Utilities|Name|MakeLiteralName "EBehaviour") (Variables|Default|GetBehaviour)))))

(event EventOnSelected
  ;[0.1469 0.1469 0.1469] Handle Lockon
  (Rendering|SetVisibility (Variables|Default|GetLockOn) true false)
  (Rendering|SetVisibility (Variables|Default|GetHealthBar) true false))

(event EventOnDeselected
  ;[0.1469 0.1469 0.1469] Handle Lockon
  (Rendering|SetVisibility (Variables|Default|GetLockOn) false false)
  (Rendering|SetVisibility (Variables|Default|GetHealthBar) false false))

(fn ConstructionScript)

(fn IsDead
  (return (Variables|Default|GetEnemyDead)))